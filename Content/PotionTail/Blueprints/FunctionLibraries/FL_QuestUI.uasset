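; FL_QuestUI is a quest UI function library that builds objective tracker widgets for a given quest.
; CreateObjectiveTrackers creates one UI_QuestObjectiveTracker per key in the quest's ObjectiveProgress map and returns them in a map under that key.
; Each widget shows the key as its name, current progress, and a required quantity read from the first stage's objectives by loop index, assuming matching order.
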(fn CreateObjectiveTrackers
  (params (InQuest :type Quest%20Base%20Object%20Reference))
  (bind _objectiveprogress (Variables|/Script/PotionTail.QuestBase|GetObjectiveProgress InQuest))
  (bind _keys (Utilities|Map|Keys _objectiveprogress))
  (for (_array_element _array_index) _keys
    (bind _returnvalue (UserInterface|CreateWidget "/Game/PotionTail/Blueprints/UI/Widgets/UI_QuestObjectiveTracker.UI_QuestObjectiveTracker_C"))
    (Utilities|Map|Add (LocalVariables|GetLocal_ObjectiveTrackers) _array_element _returnvalue)
    (Default|UpdateText _returnvalue (Utilities|Text|ToText(Name) _array_element) (.Value (Utilities|Map|Find _objectiveprogress _array_element)) (Utilities|Struct|BreakObjectiveDetails (Utilities|Array|Get(acopy) (Utilities|Struct|BreakStageDetails (Utilities|Array|Get(acopy) (Utilities|Struct|BreakQuestDetails (Variables|/Script/PotionTail.QuestBase|GetDetails InQuest)))) _array_index))))
  (return (LocalVariables|GetLocal_ObjectiveTrackers)))