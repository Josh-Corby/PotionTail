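; Dialogue component that manages a conversation's UI widget and provides a shared set of functions for driving dialogue.
; OpenConversation pushes a dialogue message through the player controller, caches the resulting UI_Dialogue widget and registers itself as its owner, while CloseConversation deactivates it.
; ProgressDialogue resets the dialogue index to -1 and calls Dialogue.
; Dialogue and the functions for adding lines, option selection, tree index and progress are empty stubs.
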(fn CloseConversation
  (Class|CommonActivatableWidget|DeactivateWidget (Variables|Default|GetDialogueWidget)))

(fn OpenConversation
  (bind _dialogueui (Class|BIPlayerController|PushDialogue(Message) (Game|GetPlayerController 0)))
  (bind _asui_dialogue (Utilities|Casting|CastToUI_Dialogue _dialogueui))
  (bind _output_get (Variables|Default|SetDialogueWidget _asui_dialogue))
  (Default|SetOwningComponent _output_get self))

(fn ProgressDialogue
  (Variables|Default|SetDialogueIndex -1)
  (CallFunction|Dialogue))

(fn AddDialogue
  (params (InSpeakerName :type Text%20%28by%20ref%29) (InDialogue :type Text%20%28by%20ref%29) (InOptionsText :type Array%20of%20Texts)))

(fn UpdateSelectedOption)

(fn RemoveDialogueProgress)

(fn SetDialogueTreeIndex)

(fn Dialogue)

(fn ClearDialogueProgress)