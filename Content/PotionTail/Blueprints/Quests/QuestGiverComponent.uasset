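; Quest giver component that offers a data-table quest to the player and hands it over when accepted.
; DisplayGiveQuest opens a quest message through the player controller, fills the UI_QuestGiver widget from the Quests row, and binds its accept event.
; On acceptance it passes QuestData to the player character, then unbinds and clears the widget.
; In-progress, ready-to-complete and completed events only print debug strings; DisplayQuest is empty.
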(event Custom|OnQuestAccepted
  (Class|PlayerInterface|AcceptQuest(Message) (Game|GetPlayerCharacter 0) (Variables|Default|GetQuestData))
  (EventDispatchers|UnbindEventfromOnQuestAccepted (Variables|Default|GetQuestGiverWidget) (EventDispatchers|CreateEvent :!event Custom|OnQuestAccepted))
  (Variables|Default|SetQuestGiverWidget 0))

(event EventDisplayGiveQuest
  (bind _outcreatedwidget (Class|BIPlayerController|DisplayQuest(Message) (Game|GetPlayerController 0)))
  (bind _asui_quest_giver (Utilities|Casting|CastToUI_QuestGiver _outcreatedwidget))
  (bind _returnvalue (Utilities|GetDataTableRow "/Game/PotionTail/Blueprints/Quests/Quests.Quests" (.RowName (Utilities|Struct|BreakDataTableRowHandle (Variables|Default|GetQuestData))))
    (:then
      (Default|SetInfo _asui_quest_giver _returnvalue)
      (Variables|Default|SetQuestGiverWidget _asui_quest_giver)
      (EventDispatchers|BindEventtoOnQuestAccepted _asui_quest_giver (EventDispatchers|CreateEvent :!event Custom|OnQuestAccepted))
      (Development|PrintString "Display quest"))))

(event EventDisplayQuestAlreadyCompleted
  (Development|PrintString "Quest already completed"))

(event EventDisplayQuestinProgress
  (Development|PrintString "quest in progress"))

(event EventDisplayQuestReadytoComplete
  (Development|PrintString "quest ready to complete"))

(fn DisplayQuest)