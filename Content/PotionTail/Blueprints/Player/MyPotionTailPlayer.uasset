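; Player character Blueprint for PotionTail that handles movement input and quest intake.
; Move input is applied along the right and forward vectors derived from the control rotation's yaw.
; AcceptQuest adds quest data to the QuestLog and tracks the new quest.
; TrackQuest notifies the QuestLog and pushes a quest tracker UI message through the player controller, then fills it with the quest's info.
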(event Custom|OnMoveInput
  (params (InX :type Float%20%28double-precision%29) (InY :type Float%20%28double-precision%29))
  (bind _returnvalue (Pawn|GetControlRotation :!class /Script/Engine.Pawn))
  (Pawn|Input|AddMovementInput (Math|Vector|GetRightVector (Math|Rotator|MakeRotator (.roll _returnvalue) 0.0 (.yaw _returnvalue))) InX false)
  (Pawn|Input|AddMovementInput (Math|Vector|GetForwardVector (Math|Rotator|MakeRotator 0.0 0.0 (.yaw (Pawn|GetControlRotation :!class /Script/Engine.Pawn)))) InY false))

(event Custom|CustomEvent
  (Utilities|FlowControl|Delay 0.1))

(fn ConstructionScript)

(fn AcceptQuest
  (params (InQuestData :type Data%20Table%20Row%20Handle%20Structure))
  (bind _returnvalue (Class|QuestLogComponent|AddNewQuest (Variables|Default|GetQuestLog) InQuestData))
  (Class|PlayerInterface|TrackQuest _returnvalue)
  (return _returnvalue))

(fn TrackQuest
  (params (InQuest :type Quest%20Base%20Object%20Reference))
  (Class|QuestLogComponent|TrackQuest (Variables|Default|GetQuestLog))
  (bind _outcreatedwidget (Class|BIPlayerController|PushQuestTrackerUI(Message) (Game|GetPlayerController 0)))
  (bind _asui_quest_tracker (Utilities|Casting|CastToUI_QuestTracker _outcreatedwidget))
  (Default|SetInfo _asui_quest_tracker InQuest))