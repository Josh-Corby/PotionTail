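; Gameplay player controller for PotionTail that links input and UI to the player pawn.
; BeginPlay adds the input mapping, caches the pawn and pushes the gameplay screen onto a layered base widget.
; Enhanced Input forwards move and interact to the pawn or opens the menu; helpers push dialogue and quest screens, and quest completion clears the quest stack.
; The interact-text binding and game-input restore are unwired, leaving menu close empty.
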(event Custom|CustomEvent
  (params (CompletedQuest :type Quest%20Base%20Object%20Reference))
  (Class|CommonActivatableWidgetContainerBase|ClearWidgets (Variables|/Game/PotionTail/Blueprints/UI/Widgets/UI_Base.UI_Base_C|GetStack_Quests (Variables|Default|GetUIBase))))

(event Custom|GameMenuClosed)

(event Custom|OnPlayerInteractableChanged
  (params (InteractableName :type Text))
  (Default|UpdateInteractText (Variables|Default|GetLinkedGameplayUI) InteractableName))

(event Input|EnhancedActionEvents|EnhancedInputActionIA_Menu
  (params (ActionValue :type Boolean) (ElapsedSeconds :type Float%20%28double-precision%29) (TriggeredSeconds :type Float%20%28double-precision%29) (InputAction :type Input%20Action%20Object%20Reference :default "/Game/PotionTail/Blueprints/Player/Input/Actions/IA_Menu.IA_Menu"))
  (:Started
    (Input|SetInputModeUIOnly self 0 "DoNotLock" false)
    (bind _pushedwidget (Default|PushMenuUI (Variables|Default|GetUIBase) "/Game/PotionTail/Blueprints/UI/Widgets/UI_GameMenu.UI_GameMenu_C"))
    (EventDispatchers|BindEventtoBPonWidgetDeactivated _pushedwidget (delegate Custom|GameMenuClosed))))

(event Input|EnhancedActionEvents|EnhancedInputActionIA_Move
  (params (ActionValue :type Vector%202D%20Structure) (ElapsedSeconds :type Float%20%28double-precision%29) (TriggeredSeconds :type Float%20%28double-precision%29) (InputAction :type Input%20Action%20Object%20Reference :default "/Game/PotionTail/Blueprints/Player/Input/Actions/IA_Move.IA_Move"))
  (Default|OnMoveInput (Variables|Default|GetLinkedPlayer) (.x ActionValue) (.y ActionValue)))

(event Input|EnhancedActionEvents|EnhancedInputActionIA_Interact
  (params (ActionValue :type Boolean) (ElapsedSeconds :type Float%20%28double-precision%29) (TriggeredSeconds :type Float%20%28double-precision%29) (InputAction :type Input%20Action%20Object%20Reference :default "/Game/PotionTail/Blueprints/Player/Input/Actions/IA_Interact.IA_Interact"))
  (:Started
    (Class|PotionTailCharacter|OnInteractInput (Variables|Default|GetLinkedPlayer))))

(event EventBeginPlay
  (bind _returnvalue (PlayerController|LocalPlayerSubsystems|GetEnhancedInputLocalPlayerSubsystem))
  (Utilities|IsValid _returnvalue
    (:Is%20Valid
      (Input|AddMappingContext _returnvalue "/Game/PotionTail/Blueprints/Player/Input/IMC_Default.IMC_Default" 0 "(bIgnoreAllPressedKeysUntilRelease=True,bForceImmediately=False,bNotifyUserSettings=False)")
      (bind _asmy_potion_tail_player (Utilities|Casting|CastToMyPotionTailPlayer (Pawn|GetControlledPawn)))
      (Variables|Default|SetLinkedPlayer _asmy_potion_tail_player)
      (bind _returnvalue_2 (UserInterface|CreateWidget "/Game/PotionTail/Blueprints/UI/Widgets/UI_Base.UI_Base_C" self))
      (bind _output_get (Variables|Default|SetUIBase _returnvalue_2))
      (UserInterface|Viewport|AddtoViewport _output_get 0)
      (bind _pushedwidget (Default|PushMainUI (Variables|Default|GetUIBase) "/Game/PotionTail/Blueprints/UI/Widgets/UI_Gameplay.UI_Gameplay_C"))
      (bind _asui_gameplay (Utilities|Casting|CastToUI_Gameplay _pushedwidget))
      (Variables|Default|SetLinkedGameplayUI _asui_gameplay)
      (EventDispatchers|BindEventtoOnQuestCompleted (Variables|/Script/PotionTail.PotionTailCharacter|GetQuestLog (Variables|Default|GetLinkedPlayer)) (delegate Custom|CustomEvent)))))

(fn ConstructionScript)

(fn DisplayQuest
  (bind _pushedwidget (Default|PushQuestUI (Variables|Default|GetUIBase) "/Game/PotionTail/Blueprints/UI/Widgets/UI_QuestGiver.UI_QuestGiver_C"))
  (return _pushedwidget))

(fn PushDialogue
  (bind _pushedwidget (Default|PushMainUI (Variables|Default|GetUIBase) "/Game/PotionTail/Blueprints/UI/Widgets/UI_Dialogue.UI_Dialogue_C"))
  (return _pushedwidget))

(fn PushQuestTrackerUI
  (bind _pushedwidget (Default|PushQuestUI (Variables|Default|GetUIBase) "/Game/PotionTail/Blueprints/UI/Widgets/UI_QuestTracker.UI_QuestTracker_C"))
  (return _pushedwidget))